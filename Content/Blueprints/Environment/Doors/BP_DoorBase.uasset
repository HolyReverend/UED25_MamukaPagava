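; BP_DoorBase is a hinged door that characters can open and close through an Interact function.
; A box collision shows a hint and enables interaction while a BP_CharacterBase overlaps it.
; One timeline, played forward or reversed, drives DoorRotator yaw up to MaxDoorOpenAngle, sets IsOpen by direction and blocks retriggering mid-swing.
; The construction script pre-rotates doors flagged as initially open.
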(event OnComponentBeginOverlap(BoxCollision)
  (params (OverlappedComponent :type Primitive%20Component%20Object%20Reference) (OtherActor :type Actor%20Object%20Reference) (OtherComp :type Primitive%20Component%20Object%20Reference) (OtherBodyIndex :type Integer) (bFromSweep :type Boolean) (SweepResult :type Hit%20Result%20Structure%20%28by%20ref%29))
  (bind _output_get (Variables|Default|SetOverlapedActor OtherActor))
  (Utilities|Casting|CastToBP_CharacterBase _output_get)
  (Rendering|SetVisibility (Variables|Default|GetHintScene) true true)
  (Variables|DoorConfigure|SetIsReadyToInteract true))

(event OnComponentEndOverlap(BoxCollision)
  (params (OverlappedComponent :type Primitive%20Component%20Object%20Reference) (OtherActor :type Actor%20Object%20Reference) (OtherComp :type Primitive%20Component%20Object%20Reference) (OtherBodyIndex :type Integer))
  (Variables|Default|SetOverlapedActor 0)
  (Utilities|Casting|CastToBP_CharacterBase OtherActor)
  (Rendering|SetVisibility (Variables|Default|GetHintScene) false true)
  (Variables|DoorConfigure|SetIsReadyToInteract false))

(event Custom|CloseDoor
  (if (not (Variables|DoorConfigure|GetInProgress))
    (if (Variables|DoorConfigure|GetIsOpen)
      (bind (_direction _openprogression) (Timeline|DoorTimeline ReverseFromEnd)
        (:Update
          (Variables|DoorConfigure|SetInProgress true)
          (Transformation|SetRelativeRotation (Variables|Default|GetDoorRotator) (Math|Rotator|MakeRotator 0.0 0.0 (* (Variables|DoorConfigure|GetMaxDoorOpenAngle) _openprogression)) false false))
        (:Finished
          (Variables|DoorConfigure|SetInProgress false)
          (switch Utilities|FlowControl|Switch|SwitchonETimelineDirection _direction
            (:Forward
              (Variables|DoorConfigure|SetIsOpen true))
            (:Backward
              (Variables|DoorConfigure|SetIsOpen false))))))))

(event Custom|OpenDoor
  (if (not (Variables|DoorConfigure|GetInProgress))
    (if (not (Variables|DoorConfigure|GetIsOpen))
      (bind (_direction _openprogression) (Timeline|DoorTimeline PlayFromStart)
        (:Update
          (Variables|DoorConfigure|SetInProgress true)
          (Transformation|SetRelativeRotation (Variables|Default|GetDoorRotator) (Math|Rotator|MakeRotator 0.0 0.0 (* (Variables|DoorConfigure|GetMaxDoorOpenAngle) _openprogression)) false false))
        (:Finished
          (Variables|DoorConfigure|SetInProgress false)
          (switch Utilities|FlowControl|Switch|SwitchonETimelineDirection _direction
            (:Forward
              (Variables|DoorConfigure|SetIsOpen true))
            (:Backward
              (Variables|DoorConfigure|SetIsOpen false))))))))

(event EventBeginPlay
  (Rendering|SetVisibility (Variables|Default|GetHintScene) false true))

(event Collision|EventActorBeginOverlap
  (params (OtherActor :type Actor%20Object%20Reference)))

(event EventTick
  (params (DeltaSeconds :type Float%20%28single-precision%29)))

(fn ConstructionScript
  (Transformation|AddRelativeRotation (Variables|Default|GetDoorRotator) (Math|Rotator|MakeRotator 0.0 0.0 (Math|Float|SelectFloat (Variables|DoorConfigure|GetMaxDoorOpenAngle) 0.0 (Variables|DoorConfigure|GetIsOpen))) false false))

(fn Interact
  (if (Variables|DoorConfigure|GetIsReadyToInteract)
    (if (Variables|DoorConfigure|GetIsOpen)
      (CallFunction|CloseDoor)
      (return true)
      (else
        (CallFunction|OpenDoor)
        (return true)))
    (else
      (return false))))
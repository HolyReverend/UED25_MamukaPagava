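; BP_AIHelper is a patrol point marker for AI, labeled in the construction script with its patrol group and point number.
; Overlap events track characters in an array and update a Vacant flag for NPCs, though end overlap removes the last actor that entered rather than the one leaving.
; A Debug flag shows the arrow, mesh and text, and rotates the label toward the player camera each tick.
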(event EventBeginPlay
  (Rendering|SetVisibility (Variables|Default|GetArrow) (Variables|Default|GetDebug) false))

(event Collision|EventActorBeginOverlap
  (params (OtherActor :type Actor%20Object%20Reference))
  (bind _output_get (Variables|Default|SetOtherActorBeginOverlap OtherActor))
  (Utilities|Casting|CastToBP_CharacterBase _output_get)
  (Utilities|Array|AddUnique (Variables|Default|GetOverlappedActors) (Variables|Default|GetOtherActorBeginOverlap))
  (Utilities|FlowControl|Sequence
    (:then_0
      (if (Variables|Default|GetDebug)
        (Utilities|Casting|CastToBP_NPCCharacter (Variables|Default|GetOtherActorBeginOverlap))
        (bind _asbp_player_character (Utilities|Casting|CastToBP_PlayerCharacter (Variables|Default|GetOtherActorBeginOverlap)))
        (Variables|Default|SetOverlappedPlayer _asbp_player_character)
        (Variables|Default|SetIsLookAtPlayerCamera true)))
    (:then_1
      (Utilities|Casting|CastToBP_NPCCharacter (Variables|Default|GetOtherActorBeginOverlap))
      (Variables|Default|SetVacant false))))

(event EventTick
  (params (DeltaSeconds :type Float%20%28single-precision%29))
  (if (Variables|Default|GetDebug)
    (CallFunction|LookingatPlayerCamera)))

(event Collision|EventActorEndOverlap
  (params (OtherActor :type Actor%20Object%20Reference))
  (bind _output_get (Variables|Default|SetOtherActorEndOverlap OtherActor))
  (Utilities|Casting|CastToBP_CharacterBase _output_get)
  (bind _returnvalue (Utilities|Array|RemoveItem (Variables|Default|GetOverlappedActors) (Variables|Default|GetOtherActorBeginOverlap)))
  (if _returnvalue
    (Utilities|FlowControl|Sequence
      (:then_0
        (if (Variables|Default|GetDebug)
          (Utilities|Casting|CastToBP_NPCCharacter (Variables|Default|GetOtherActorBeginOverlap))
          (Variables|Default|SetOverlappedPlayer 0)
          (Variables|Default|SetIsLookAtPlayerCamera false)))
      (:then_1
        (Utilities|Casting|CastToBP_NPCCharacter (Variables|Default|GetOtherActorBeginOverlap))
        (if (Utilities|Array|IsValidIndex (Variables|Default|GetOverlappedActors))
          (Variables|Default|SetVacant false)
          (else
            (Variables|Default|SetVacant true)))))))

(fn ConstructionScript
  (if (!= (Variables|Default|GetPatrollGroup) 0)
    (Rendering|Components|TextRender|SetText (Variables|Default|GetTextRender) (Utilities|Text|FormatText "Group {A} | Point {B}" (Variables|Default|GetPatrollGroup) (Variables|Default|GetPatrollPointNumbeer)))
    (else
      (Rendering|Components|TextRender|SetText (Variables|Default|GetTextRender) (Utilities|Text|FormatText "Set Patroll group")))))

(fn LookingatPlayerCamera
  (bind _asbp_player_character (Utilities|Casting|CastToBP_PlayerCharacter (Game|Player|GetPlayerPawn 0)))
  (LocalVariables|SetL_CameraLocation (Transformation|GetWorldLocation (Variables|/Game/Blueprints/Characters/Player/BP_PlayerCharacter.BP_PlayerCharacter_C|GetCamera _asbp_player_character)))
  (Transformation|SetWorldRotation (Variables|Default|GetTextRender) (Math|Rotator|FindLookatRotation (Transformation|GetWorldLocation (Variables|Default|GetTextRender)) (LocalVariables|GetL_CameraLocation)) false false))
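; Base actor for interactable items that a character can pick up into a backpack.
; Overlap events track the nearby character, enable interaction and show a text prompt, which Tick turns toward the BP_PlayerCharacter camera.
; Interact passes the character's BP_BackpackComponent to PutIntoBackpack, an empty hook here, and returns true on every path.
; AfterUse destroys the actor but is not called within this Blueprint.
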(event EventBeginPlay
  (Rendering|SetVisibility (Variables|Default|GetTextRender) false false))

(event Collision|EventActorBeginOverlap
  (params (OtherActor :type Actor%20Object%20Reference))
  (bind _ascharacter (Utilities|Casting|CastToCharacter OtherActor))
  (Variables|Default|SetCharacter%20in%20Box _ascharacter)
  (Rendering|SetVisibility (Variables|Default|GetTextRender) true false)
  (Variables|Default|SetIsReadyToInteract true)
  (Variables|Default|SetIsLookAtPlayerCamera true))

(event EventTick
  (params (DeltaSeconds :type Float%20%28single-precision%29))
  (CallFunction|LookingatPlayerCamera))

(event Collision|EventActorEndOverlap
  (params (OtherActor :type Actor%20Object%20Reference))
  (Utilities|Casting|CastToCharacter OtherActor)
  (Variables|Default|SetCharacter%20in%20Box 0)
  (Rendering|SetVisibility (Variables|Default|GetTextRender) false false)
  (Variables|Default|SetIsReadyToInteract false)
  (Variables|Default|SetIsLookAtPlayerCamera false))

(fn ConstructionScript)

(fn LookingatPlayerCamera
  (if (Variables|Default|GetIsLookAtPlayerCamera)
    (bind _character_in_box (Variables|Default|GetCharacter%20in%20Box)
      (:then
        (bind _asbp_player_character (Utilities|Casting|CastToBP_PlayerCharacter _character_in_box))
        (LocalVariables|SetL_CameraLocation (Transformation|GetWorldLocation (Variables|/Game/Blueprints/Characters/Player/BP_PlayerCharacter.BP_PlayerCharacter_C|GetCamera _asbp_player_character)))
        (Transformation|SetWorldRotation (Variables|Default|GetTextRender) (Math|Rotator|FindLookatRotation (Transformation|GetWorldLocation (Variables|Default|GetTextRender)) (LocalVariables|GetL_CameraLocation)) false false))
      (:else))))

(fn PutIntoBackpack
  (params (InBackpack :type BP%20Backpack%20Component%20Object%20Reference)))

(fn AfterUse
  (Actor|DestroyActor))

(fn Interact
  (if (Variables|Default|GetIsReadyToInteract)
    (bind _character_in_box (Variables|Default|GetCharacter%20in%20Box)
      (:then
        (Utilities|IsValid (Actor|GetComponentbyClass _character_in_box "/Game/Blueprints/Components/BP_BackpackComponent.BP_BackpackComponent_C")
          (:Is%20Valid
            (CallFunction|PutIntoBackpack (Actor|GetComponentbyClass _character_in_box "/Game/Blueprints/Components/BP_BackpackComponent.BP_BackpackComponent_C"))
            (return true))
          (:Is%20Not%20Valid
            (return true))))
      (:else
        (return true)))
    (else
      (return true))))
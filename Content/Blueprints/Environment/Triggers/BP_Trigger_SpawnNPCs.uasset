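; Overlap trigger that starts NPC spawning through its linked spawners when the player character sets it off.
; On actor begin overlap it runs the parent handler, then continues only if the cast to BP_PlayerCharacter succeeds.
; It then loops over the NPCSpawners array and calls StartSpawnNPCs on each entry.
; The Blueprint itself has no guard against firing again on later overlaps.
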(event EventBeginPlay
  (|CallParentFunction) ; This node is disabled and will not be called.\nDrag off pins to build functionality.
)

(event Collision|EventActorBeginOverlap
  (params (OtherActor :type Actor%20Object%20Reference))
  (|CallParentFunction OtherActor)
  (Utilities|Casting|CastToBP_PlayerCharacter (Variables|Default|GetOverlappedActor))
  (for _array_element (Variables|Default|GetNPCSpawners)
    (Default|StartSpawnNPCs _array_element)))

(event EventTick
  (params (DeltaSeconds :type Float%20%28single-precision%29))
  (|CallParentFunction DeltaSeconds) ; This node is disabled and will not be called.\nDrag off pins to build functionality.
)

(fn ConstructionScript
  (|CallParentFunction))
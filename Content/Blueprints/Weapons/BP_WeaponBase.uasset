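; BP_WeaponBase is a base weapon Blueprint that holds stats, active state and shoot input, with firing currently only a debug print.
; ConfigureWeaponStats loads the named DT_WeaponStats row, fills current rounds and scales damage by the owner's BP_MainStatsComponent damage multiplier.
; ShootProcess stores the trigger state, and Tick calls Shooting while active, printing damage every frame the trigger is held without consuming rounds.
; Interact is a stub returning false.
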(event EventBeginPlay)

(event Collision|EventActorBeginOverlap
  (params (OtherActor :type Actor%20Object%20Reference)))

(event EventTick
  (params (DeltaSeconds :type Float%20%28single-precision%29))
  (if (Variables|Configuration|GetIsWeaponActive)
    (Shoot|Shooting)))

(event EventShootProcess
  (params (InProcess :type Boolean))
  (Shoot|ShootInputRecived InProcess))

(fn ConstructionScript)

(fn ConfigureWeaponStats
  (params (InWeaponName :type Name))
  (bind _returnvalue (Components|GetOwner))
  (bind _returnvalue_2 (Actor|GetComponentbyClass _returnvalue "/Game/Blueprints/Components/BP_MainStatsComponent.BP_MainStatsComponent_C"))
  (Variables|Configuration|SetWeaponName InWeaponName)
  (if (Utilities|Name|NotEqual(Name) (Variables|Configuration|GetWeaponName) "None")
    (bind _returnvalue_3 (Utilities|GetDataTableRow "/Game/Data/DT_WeaponStats.DT_WeaponStats" (Variables|Configuration|GetWeaponName))
      (:then
        (Variables|Configuration|SetWeaponStats _returnvalue_3)
        (Variables|Configuration|SetRoundsCurrent (Utilities|Struct|BreakSTRUCT_WeaponStats (Variables|Configuration|GetWeaponStats)))
        (Variables|Configuration|SetDamageCurrent (Utilities|Struct|BreakSTRUCT_WeaponStats (Variables|Configuration|GetWeaponStats)))
        (Utilities|IsValid _returnvalue
          (:Is%20Valid
            (Utilities|IsValid _returnvalue_2
              (:Is%20Valid
                (Variables|Configuration|SetDamageCurrent (Math|Float|Truncate (* (Variables|Configuration|GetDamageCurrent) (Utilities|Struct|BreakSTRUCT_MainStats (Variables|/Game/Blueprints/Components/BP_MainStatsComponent.BP_MainStatsComponent_C|GetMainStatsStructure _returnvalue_2))))))))))
      (:RowNotFound
        (Development|PrintString "Configure Weapon stats failed: Current name is not found in Data Table")))
    (else
      (Development|PrintString "Configure Weapon stats failed: Current name is invalid"))))

(fn Shooting
  (if (Variables|Default|GetInProcess)
    (Development|PrintString (Utilities|String|Append "Banq for" (Utilities|String|ToString(Integer) (Variables|Configuration|GetDamageCurrent)) "damage!"))))

(fn ShootInputRecived
  (params (InProcess :type Boolean))
  (Variables|Default|SetInProcess InProcess))

(fn ActivateWeapon
  (params (InActivation :type Boolean))
  (Variables|Configuration|SetIsWeaponActive InActivation))

(fn Interact
  (return false))